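; Numbered track checkpoint that HoverCars must pass in order, also serving as their respawn point.
; The Initialise event finds the checkpoint with the next number, stores it as NextCP and turns PivotArrow toward it.
; On overlap, a car expecting this number advances its NextCheckpoint, a sound plays, and its respawn transform moves here, raised by the car's hover distance.
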(event Custom|Initialise
  (bind _outactors (Actor|GetAllActorsOfClass "Checkpoint_BP_C"))
  (bind _array_element (Utilities|Array|ForEachLoopwithBreak _outactors :!label _label)
    (:LoopBody
      (if (== (- (Variables|Checkpoint_BP_C|GetCheckpointNum _array_element) 1) (Variables|Default|GetCheckpointNum))
        (Variables|Default|SetNextCP _array_element)
        (Transformation|SetRelativeRotation (Variables|Default|GetPivot%20Arrow) (Math|Rotator|MakeRotfromX (Math|Transform|InverseTransformLocation (Transformation|GetWorldTransform (Variables|Default|GetSphere)) (Transformation|GetActorLocation _array_element))) false false)
        (goto _label Break)))))

(event EventBeginPlay)

(event Collision|EventActorBeginOverlap
  (params (OtherActor :type Actor%20Object%20Reference))
  (bind _ashover_car (Utilities|Casting|CastToHoverCar OtherActor))
  (if (== (Variables|/Game/HoverCar/HoverCar.HoverCar_C|GetNextCheckpoint _ashover_car) (Variables|Default|GetCheckpointNum))
    (Variables|/Game/HoverCar/HoverCar.HoverCar_C|SetNextCheckpoint _ashover_car (+ (Variables|/Game/HoverCar/HoverCar.HoverCar_C|GetNextCheckpoint _ashover_car) 1))
    (Audio|PlaySoundatLocation "/Engine/EditorSounds/GamePreview/StartPlayInEditor_Cue.StartPlayInEditor_Cue" (Transformation|GetActorLocation) "0, 0, 0" 1.0 1.0 0.0 0 0 0 0)
    ;[1 1 1] Set respawn location
    (Variables|/Game/HoverCar/HoverCar.HoverCar_C|SetRespawnTransform _ashover_car (Math|Transform|MakeTransform (+ (Transformation|GetActorLocation) (Math|Vector|MakeVector 0.0 0.0 (Variables|/Game/HoverCar/HoverCar.HoverCar_C|GetHoverDistance _ashover_car))) (Transformation|GetActorRotation) (Transformation|GetActorScale3D _ashover_car)))))

(fn ConstructionScript)